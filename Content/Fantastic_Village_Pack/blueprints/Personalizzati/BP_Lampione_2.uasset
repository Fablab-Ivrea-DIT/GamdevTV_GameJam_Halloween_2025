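; BP_Lampione_2 is a street lamp Blueprint whose light flickers continuously from BeginPlay.
; The Flick event randomly picks a bright or dim intensity range, then sets the light to a random value within it.
; It re-arms a short fixed-interval timer that calls Flick again, so the flicker repeats without using Tick.
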(event `self.ReceiveBeginPlay`
  (`self.Flick`))

(event `self.ReceiveTick`
  (params (DeltaSeconds :type "Float (single-precision)")))

(event `Flick`
  (if (`KismetMathLibrary.RandomBool`)
    (`LightComponent.SetIntensity` (`self.Light`) (`KismetMathLibrary.RandomFloatInRange` 3000.0 5000.0))
    (else
      (`LightComponent.SetIntensity` (`self.Light`) (`KismetMathLibrary.RandomFloatInRange` 20.0 100.0))))
  (`KismetSystemLibrary.K2_SetTimerDelegate` (delegate `_Flick`) 0.1))

(event `_Flick`
  (`self.Flick`))

(fn `UserConstructionScript`)