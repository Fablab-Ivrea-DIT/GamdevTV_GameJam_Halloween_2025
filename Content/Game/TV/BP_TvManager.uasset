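; BP_TvManager drives the in-game TV screen and the UI shown with it for the main menu and story sequences.
; On BeginPlay it puts a dynamic static-noise material on the TV and opens the menu widget.
; Update checks BP_LevelInstance's StartStory flag, swaps in a light static material, and spawns WBP_Story with that material plus the texts and scenes for the current chapter.
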(event `Update`
  (bind _asbp_level_instance (cast `/Game/Game/GameModesAndStuff/BP_LevelInstance` (`GameplayStatics.GetGameInstance`)))
  (if (`/Game/Game/GameModesAndStuff/BP_LevelInstance.StartStory` _asbp_level_instance)
    (bind _returnvalue (`KismetMaterialLibrary.CreateDynamicMaterialInstance` "/Game/Game/TV/M_StaticLIGHT.M_StaticLIGHT"))
    (set `self.Material` _returnvalue)
    (`PrimitiveComponent.SetMaterial` (`StaticMeshActor.StaticMeshComponent` (`self.TV`)) 1 (`self.Material`))
    (switch `int` (`/Game/Game/GameModesAndStuff/BP_LevelInstance.Chapter` _asbp_level_instance)
      (:`0`
        (bind _returnvalue_2 (`|CreateWidget` "/Game/Game/TV/UIs/WBP_Story.WBP_Story_C" null (`self.Material`) (`self.TextsONE`) (`self.ScenesONE`)))
        (`UserWidget.AddToViewport` _returnvalue_2 0))
      (:`1`
        (bind _returnvalue_3 (`|CreateWidget` "/Game/Game/TV/UIs/WBP_Story.WBP_Story_C" null (`self.Material`) (`self.TextsTWO`) (`self.ScenesTWO`)))
        (`UserWidget.AddToViewport` _returnvalue_3 0)))))

(event `self.ReceiveBeginPlay`
  (bind _returnvalue (`KismetMaterialLibrary.CreateDynamicMaterialInstance` "/Game/Game/TV/M_Static.M_Static"))
  (set `self.Material` _returnvalue)
  (`PrimitiveComponent.SetMaterial` (`StaticMeshActor.StaticMeshComponent` (`self.TV`)) 1 (`self.Material`))
  (bind _returnvalue_2 (`|CreateWidget` "/Game/Game/TV/UIs/WBP_Menu.WBP_Menu_C"))
  (`UserWidget.AddToViewport` _returnvalue_2 0))

(fn `UserConstructionScript`)