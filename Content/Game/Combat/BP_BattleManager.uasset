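; BP_BattleManager is the combat manager that moves the player and an enemy from the world into a battle arena.
; InitializeCombat disables player input and scans all BP_BattleArena actors for the one closest to the player.
; It teleports both combatants to opposite sides of that arena's center, offset by its Distance, then cubic-blends the camera view to the arena.
; Only this setup is implemented, with no turn or end-of-combat logic.
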(event `self.ReceiveBeginPlay`)

(event `InitializeCombat`
  (params (Enemy :type "Actor Object Reference") (Player :type "Actor Object Reference"))
  (bind _arenachosen (`self.ArenaChosen`))
  (bind _arenachosen_2 (`self.ArenaChosen`))
  (`self.DisableInput` (`GameplayStatics.GetPlayerPawn` 0) (`GameplayStatics.GetPlayerController` 0))
  (bind _outactors (`GameplayStatics.GetAllActorsOfClass` "/Game/Game/Combat/BP_BattleArena.BP_BattleArena_C"))
  (for _array_element _outactors
    (bind _returnvalue (`self.GetDistanceTo` Player _array_element))
    (if (< _returnvalue (`self.ClosestDistance`))
      (set `self.ClosestDistance` _returnvalue)
      (set `self.ArenaChosen` _array_element)))
  (`self.K2_TeleportTo` Player (+ (`self.K2_GetActorLocation` _arenachosen_2) (`KismetMathLibrary.MakeVector` (`/Game/Game/Combat/BP_BattleArena.Distance` _arenachosen_2) 0.0 90.0)) (struct :`Yaw` 180.0))
  (`self.K2_TeleportTo` :`self` Enemy :`DestLocation` (- (`self.K2_GetActorLocation` _arenachosen) (`KismetMathLibrary.MakeVector` (`/Game/Game/Combat/BP_BattleArena.Distance` _arenachosen) 0.0 -90.0)))
  (`PlayerController.SetViewTargetWithBlend` (`GameplayStatics.GetPlayerController` 0) (`self.ArenaChosen`) 5.0 "VTBlend_Cubic" 0.0 false))

(fn `UserConstructionScript`)