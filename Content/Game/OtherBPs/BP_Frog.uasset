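; BP_Frog is a talkable frog actor that exists only in Chapter 1 and destroys itself in other chapters.
; On BeginPlay it checks the chapter in BP_LevelInstance and copies all rows of its Dialogues data table into an array.
; Its sphere overlap shows or hides a widget as BP_Boy enters or leaves.
; Talk opens WBP_DialogueBox with those lines, switches to UI-only input with a cursor, then destroys the frog, making it one-time.
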(event `self.ReceiveBeginPlay`
  (bind _asbp_level_instance (cast `/Game/Game/GameModesAndStuff/BP_LevelInstance` (`GameplayStatics.GetGameInstance`)))
  (if (== (`/Game/Game/GameModesAndStuff/BP_LevelInstance.Chapter` _asbp_level_instance) 1)
    (bind _outrownames (`DataTableFunctionLibrary.GetDataTableRowNames` (`self.Dialogues`)))
    (for _array_element _outrownames
      (bind _returnvalue (`|GetDataTableRow` (`self.Dialogues`) _array_element)
        (:`then`
          (`KismetArrayLibrary.Array_Add` (`self.DialoguesReady`) _returnvalue))))
    (else
      (`self.K2_DestroyActor`))))

(event `self.Sphere.OnComponentBeginOverlap`
  (params (OverlappedComponent :type "PrimitiveComponent Object Reference") (OtherActor :type "Actor Object Reference") (OtherComp :type "PrimitiveComponent Object Reference") (OtherBodyIndex :type Integer) (bFromSweep :type Boolean) (SweepResult :type "HitResult Structure (by ref)"))
  (cast `/Game/Game/Characters/BP_Boy` OtherActor)
  (`SceneComponent.SetVisibility` (`self.Widget`) true false))

(event `self.ReceiveTick`
  (params (DeltaSeconds :type "Float (single-precision)")))

(event `self.Sphere.OnComponentEndOverlap`
  (params (OverlappedComponent :type "PrimitiveComponent Object Reference") (OtherActor :type "Actor Object Reference") (OtherComp :type "PrimitiveComponent Object Reference") (OtherBodyIndex :type Integer))
  (cast `/Game/Game/Characters/BP_Boy` OtherActor)
  (`SceneComponent.SetVisibility` (`self.Widget`) false false))

(event `self.Talk`
  (bind _returnvalue (`GameplayStatics.GetPlayerController` 0))
  (bind _returnvalue_2 (`|CreateWidget` "/Game/Dialogue/WBP_DialogueBox.WBP_DialogueBox_C" (`GameplayStatics.GetPlayerController` 0) (`self.DialoguesReady`) false null "/Engine/EngineSounds/1kSineTonePing.1kSineTonePing"))
  (bind _output_get (set `self.DialogueShown` _returnvalue_2))
  (`/Game/Dialogue/WBP_DialogueBox.UpdateDialogue` _output_get)
  (`UserWidget.AddToViewport` _output_get 0)
  (set `PlayerController.bShowMouseCursor` true _returnvalue)
  (`WidgetBlueprintLibrary.SetInputMode_UIOnlyEx` _returnvalue null "DoNotLock" true)
  (`self.K2_DestroyActor`)
  (set `self.ShouldPick` false)
  (`self.SetActorHiddenInGame` true))

(fn `UserConstructionScript`)