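; BP_Kitty2 is a quest NPC cat that sends the player after a wool ball held by the graveyard monster, and destroys itself past chapter 2.
; It loads the current dialogue DataTable into an array for a dialogue widget, and toggles a widget when BP_Boy enters or leaves its sphere.
; Talk branches on QuestDone, either priming BP_Monster for battle or revealing FabricBalls and advancing BP_Skelly's dialogue, updating quest text through the game mode.
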(event `ResetDialogues`
  (`KismetArrayLibrary.Array_Clear` (`self.DialoguesReady`))
  (bind _asbp_level_instance (cast `/Game/Game/GameModesAndStuff/BP_LevelInstance` (`GameplayStatics.GetGameInstance`) :!label _label))
  (if (>= 2 (`/Game/Game/GameModesAndStuff/BP_LevelInstance.Chapter` _asbp_level_instance))
    (bind _outrownames (`DataTableFunctionLibrary.GetDataTableRowNames` (`|GetArrayItem` (`self.Dialogues`) (`self.DialogueIndex`))))
    (for _array_element _outrownames
      (bind _returnvalue (`|GetDataTableRow` (`|GetArrayItem` (`self.Dialogues`) (`self.DialogueIndex`)) _array_element)
        (:`then`
          (`KismetArrayLibrary.Array_Add` (`self.DialoguesReady`) _returnvalue))))
    (else
      (`self.K2_DestroyActor`))))

(event `self.ReceiveBeginPlay`
  (goto _label))

(event `self.Sphere.OnComponentBeginOverlap`
  (params (OverlappedComponent :type "PrimitiveComponent Object Reference") (OtherActor :type "Actor Object Reference") (OtherComp :type "PrimitiveComponent Object Reference") (OtherBodyIndex :type Integer) (bFromSweep :type Boolean) (SweepResult :type "HitResult Structure (by ref)"))
  (cast `/Game/Game/Characters/BP_Boy` OtherActor)
  (`SceneComponent.SetVisibility` (`self.Widget`) true false))

(event `self.Sphere.OnComponentEndOverlap`
  (params (OverlappedComponent :type "PrimitiveComponent Object Reference") (OtherActor :type "Actor Object Reference") (OtherComp :type "PrimitiveComponent Object Reference") (OtherBodyIndex :type Integer))
  (cast `/Game/Game/Characters/BP_Boy` OtherActor)
  (`SceneComponent.SetVisibility` (`self.Widget`) false false))

(event `/Game/Dialogue/BI_DialogueInterface.Talk`
  (if (`self.QuestDone`)
    (`SceneComponent.SetVisibility` (`self.fabric_balls`) true false)
    (set `self.DialogueIndex` 1)
    (`self.ResetDialogues`)
    (`self.StartDialogue`)
    (bind _returnvalue (`GameplayStatics.GetActorOfClass` "/Game/Game/Characters/BP_Skelly.BP_Skelly_C"))
    (set `/Game/Game/Characters/BP_Skelly.DialogueIndex` 1 _returnvalue)
    (`/Game/Game/Characters/BP_Skelly.ResetDialogues` _returnvalue)
    (bind _asbp_level_instance (cast `/Game/Game/GameModesAndStuff/BP_LevelInstance` (`GameplayStatics.GetGameInstance`)))
    (`KismetArrayLibrary.Array_Set` (`/Game/Game/GameModesAndStuff/BP_LevelInstance.QuestTexts` _asbp_level_instance) (`/Game/Game/GameModesAndStuff/BP_LevelInstance.Chapter` _asbp_level_instance) "Meet other graveyard residents! Maybe an old, grumpy skeleton?")
    (bind _asgm_basic_gameplay (cast `/Game/Game/GameModesAndStuff/GM_BasicGameplay` (`GameplayStatics.GetGameMode`)))
    (`/Game/Game/GameModesAndStuff/GM_BasicGameplay.ChangeQuestDeleg` _asgm_basic_gameplay)
    (else
      (`self.StartDialogue`)
      (if (not (`self.QuestDone`))
        (bind _returnvalue_2 (`GameplayStatics.GetActorOfClass` "/Game/Game/Enemies/BP_Monster.BP_Monster_C"))
        (set `/Game/Game/Enemies/BP_Monster.DialogueIndex` 1 _returnvalue_2)
        (`/Game/Game/Enemies/BP_Monster.ToggleMarkerVisibility` _returnvalue_2)
        (`/Game/Game/Enemies/BP_Monster.ResetDialogues` _returnvalue_2)
        (set `/Game/Game/Enemies/BP_Monster.StartBattle` true _returnvalue_2)
        (bind _asbp_level_instance_2 (cast `/Game/Game/GameModesAndStuff/BP_LevelInstance` (`GameplayStatics.GetGameInstance`)))
        (`KismetArrayLibrary.Array_Set` (`/Game/Game/GameModesAndStuff/BP_LevelInstance.QuestTexts` _asbp_level_instance_2) (`/Game/Game/GameModesAndStuff/BP_LevelInstance.Chapter` _asbp_level_instance_2) "Recover Frisky wool ball from the evil monster in the graveyard!")
        (bind _asgm_basic_gameplay_2 (cast `/Game/Game/GameModesAndStuff/GM_BasicGameplay` (`GameplayStatics.GetGameMode`)))
        (`/Game/Game/GameModesAndStuff/GM_BasicGameplay.ChangeQuestDeleg` _asgm_basic_gameplay_2)))))

(event `StartDialogue`
  (bind _returnvalue (`GameplayStatics.GetPlayerController` 0))
  (bind _returnvalue_2 (`|CreateWidget` "/Game/Dialogue/WBP_DialogueBox.WBP_DialogueBox_C" (`GameplayStatics.GetPlayerController` 0) (`self.DialoguesReady`) false null))
  (bind _output_get (set `self.DialogueShown` _returnvalue_2))
  (`/Game/Dialogue/WBP_DialogueBox.UpdateDialogue` _output_get)
  (`UserWidget.AddToViewport` _output_get 0)
  (set `PlayerController.bShowMouseCursor` true _returnvalue)
  (`WidgetBlueprintLibrary.SetInputMode_UIOnlyEx` _returnvalue null "DoNotLock" true))

(fn `UserConstructionScript`)