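; BP_NPC is an NPC that opens a dialogue box when BP_Ty enters its sphere or when Talk is called.
; BeginPlay copies every row of the Dialogues data table into DialoguesReady, which StartDialogue passes to a new WBP_DialogueBox.
; StartDialogue also shows the cursor and switches to UI-only input.
; Any actor leaving the sphere removes the box and restores game-only input, as end overlap has no cast check.
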(event `self.ReceiveBeginPlay`
  (bind _outrownames (`DataTableFunctionLibrary.GetDataTableRowNames` (`self.Dialogues`)))
  (for _array_element _outrownames
    (bind _returnvalue (`|GetDataTableRow` (`self.Dialogues`) _array_element)
      (:`then`
        (`KismetArrayLibrary.Array_Add` (`self.DialoguesReady`) _returnvalue)))))

(event `/Game/Dialogue/BI_DialogueInterface.Talk`
  (`self.StartDialogue`))

(event `StartDialogue`
  (bind _returnvalue (`GameplayStatics.GetPlayerController` 0))
  (bind _returnvalue_2 (`|CreateWidget` "/Game/Dialogue/WBP_DialogueBox.WBP_DialogueBox_C" (`GameplayStatics.GetPlayerController` 0) (`self.DialoguesReady`)))
  (bind _output_get (set `self.DialogueShown` _returnvalue_2))
  (`/Game/Dialogue/WBP_DialogueBox.UpdateDialogue` _output_get)
  (`UserWidget.AddToViewport` _output_get 0)
  (set `PlayerController.bShowMouseCursor` true _returnvalue)
  (`WidgetBlueprintLibrary.SetInputMode_UIOnlyEx` _returnvalue null "DoNotLock" true))

(event `self.Sphere.OnComponentBeginOverlap`
  (params (OverlappedComponent :type "PrimitiveComponent Object Reference") (OtherActor :type "Actor Object Reference") (OtherComp :type "PrimitiveComponent Object Reference") (OtherBodyIndex :type Integer) (bFromSweep :type Boolean) (SweepResult :type "HitResult Structure (by ref)"))
  (cast `/Game/Game/Characters/BP_Ty` OtherActor)
  (`self.StartDialogue`))

(event `self.Sphere.OnComponentEndOverlap`
  (params (OverlappedComponent :type "PrimitiveComponent Object Reference") (OtherActor :type "Actor Object Reference") (OtherComp :type "PrimitiveComponent Object Reference") (OtherBodyIndex :type Integer))
  (bind _returnvalue (`GameplayStatics.GetPlayerController` 0))
  (`Widget.RemoveFromParent` (`self.DialogueShown`))
  (set `PlayerController.bShowMouseCursor` false _returnvalue)
  (`WidgetBlueprintLibrary.SetInputMode_GameOnly` _returnvalue))

(event `CustomEvent`
  (`KismetSystemLibrary.PrintString` "Hello"))

(fn `UserConstructionScript`)