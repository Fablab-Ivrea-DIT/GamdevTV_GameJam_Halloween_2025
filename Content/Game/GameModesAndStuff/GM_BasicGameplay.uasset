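; Gameplay game mode that sets up each of three story chapters, using the Chapter stored in the BP_LevelInstance game instance.
; BeginPlay moves the player to the chapter's start, sets day or dawn via BP_DayManager, then shows that chapter's DataTable dialogue in WBP_DialogueBox and the quest text in BP_GameUI.
; Cutscene events advance Chapter and open TVScene; SaveTemp and LoadTemp store and restore player position through the game instance.
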(event `StartThirdDialogue`
  (bind _returnvalue (`GameplayStatics.GetPlayerController` 0))
  (bind _outrownames (`DataTableFunctionLibrary.GetDataTableRowNames` (`|GetArrayItem` (`self.Dialogues`) 2)))
  (for _array_element _outrownames
    (bind _returnvalue_2 (`|GetDataTableRow` (`|GetArrayItem` (`self.Dialogues`) 2) _array_element)
      (:`then`
        (`KismetArrayLibrary.Array_Add` (`self.DialoguesReady`) _returnvalue_2))))
  (bind _returnvalue_3 (`|CreateWidget` "/Game/Dialogue/WBP_DialogueBox.WBP_DialogueBox_C" (`GameplayStatics.GetPlayerController` 0) (`self.DialoguesReady`) false null))
  (bind _output_get (set `self.DialogueShown` _returnvalue_3))
  (`/Game/Dialogue/WBP_DialogueBox.UpdateDialogue` _output_get)
  (`UserWidget.AddToViewport` _output_get 0)
  (set `PlayerController.bShowMouseCursor` true _returnvalue)
  (`WidgetBlueprintLibrary.SetInputMode_UIOnlyEx` _returnvalue null "DoNotLock" true))

(event `StartSecondDialogue`
  (bind _returnvalue (`GameplayStatics.GetPlayerController` 0))
  (bind _outrownames (`DataTableFunctionLibrary.GetDataTableRowNames` (`|GetArrayItem` (`self.Dialogues`) 1)))
  (for _array_element _outrownames
    (bind _returnvalue_2 (`|GetDataTableRow` (`|GetArrayItem` (`self.Dialogues`) 1) _array_element)
      (:`then`
        (`KismetArrayLibrary.Array_Add` (`self.DialoguesReady`) _returnvalue_2))))
  (bind _returnvalue_3 (`|CreateWidget` "/Game/Dialogue/WBP_DialogueBox.WBP_DialogueBox_C" (`GameplayStatics.GetPlayerController` 0) (`self.DialoguesReady`) false null))
  (bind _output_get (set `self.DialogueShown` _returnvalue_3))
  (`/Game/Dialogue/WBP_DialogueBox.UpdateDialogue` _output_get)
  (`UserWidget.AddToViewport` _output_get 0)
  (set `PlayerController.bShowMouseCursor` true _returnvalue)
  (`WidgetBlueprintLibrary.SetInputMode_UIOnlyEx` _returnvalue null "DoNotLock" true))

(event `StartFirstDialogue`
  (bind _returnvalue (`GameplayStatics.GetPlayerController` 0))
  (bind _outrownames (`DataTableFunctionLibrary.GetDataTableRowNames` (`|GetArrayItem` (`self.Dialogues`))))
  (for _array_element _outrownames
    (bind _returnvalue_2 (`|GetDataTableRow` (`|GetArrayItem` (`self.Dialogues`)) _array_element)
      (:`then`
        (`KismetArrayLibrary.Array_Add` (`self.DialoguesReady`) _returnvalue_2))))
  (bind _returnvalue_3 (`|CreateWidget` "/Game/Dialogue/WBP_DialogueBox.WBP_DialogueBox_C" (`GameplayStatics.GetPlayerController` 0) (`self.DialoguesReady`) false null))
  (bind _output_get (set `self.DialogueShown` _returnvalue_3))
  (`/Game/Dialogue/WBP_DialogueBox.UpdateDialogue` _output_get)
  (`UserWidget.AddToViewport` _output_get 0)
  (set `PlayerController.bShowMouseCursor` true _returnvalue)
  (`WidgetBlueprintLibrary.SetInputMode_UIOnlyEx` _returnvalue null "DoNotLock" true))

(event `self.ReceiveBeginPlay`
  (`self.Load`)
  (bind _asbp_level_instance (cast `/Game/Game/GameModesAndStuff/BP_LevelInstance` (`GameplayStatics.GetGameInstance`)))
  (switch `int` (`/Game/Game/GameModesAndStuff/BP_LevelInstance.Chapter` _asbp_level_instance)
    (:`0`
      (`self.StartFirstDialogue`))
    (:`1`
      (`self.StartSecondDialogue`))
    (:`2`
      (`self.StartThirdDialogue`)))
  (bind _returnvalue (`|CreateWidget` "/Game/Game/UI/BP_GameUI.BP_GameUI_C" (`GameplayStatics.GetPlayerController` 0)))
  (`UserWidget.AddToViewport` _returnvalue 0)
  (set `self.UIQuest` _returnvalue)
  (`self.ChangeQuestDeleg`))

(event `ChangeQuestDeleg`
  (bind _asbp_level_instance (cast `/Game/Game/GameModesAndStuff/BP_LevelInstance` (`GameplayStatics.GetGameInstance`)))
  (`/Game/Game/UI/BP_GameUI.ChangeQuest` (`self.UIQuest`) (`|GetArrayItem` (`/Game/Game/GameModesAndStuff/BP_LevelInstance.QuestTexts` _asbp_level_instance) (`/Game/Game/GameModesAndStuff/BP_LevelInstance.Chapter` _asbp_level_instance))))

(event `SaveTemp`
  (bind _asbp_level_instance (cast `/Game/Game/GameModesAndStuff/BP_LevelInstance` (`GameplayStatics.GetGameInstance`)))
  (set `/Game/Game/GameModesAndStuff/BP_LevelInstance.PlayerPosition` (`self.K2_GetActorLocation` (`Controller.K2_GetPawn` (`GameplayStatics.GetPlayerController` 0))) _asbp_level_instance))

(event `LoadTemp`
  (bind _asbp_level_instance (cast `/Game/Game/GameModesAndStuff/BP_LevelInstance` (`GameplayStatics.GetGameInstance`)))
  (`self.K2_SetActorLocation` (`GameplayStatics.GetPlayerCharacter` 0) (`/Game/Game/GameModesAndStuff/BP_LevelInstance.PlayerPosition` _asbp_level_instance) false false))

(event `Load`
  (bind _returnvalue (`Controller.K2_GetPawn` (`GameplayStatics.GetPlayerController` 0)))
  (bind _asbp_level_instance (cast `/Game/Game/GameModesAndStuff/BP_LevelInstance` (`GameplayStatics.GetGameInstance`)))
  (bind _chapter (`/Game/Game/GameModesAndStuff/BP_LevelInstance.Chapter` _asbp_level_instance))
  (switch `int` _chapter
    (:`0`
      (bind _output (`|GetArrayItem` (`/Game/Game/GameModesAndStuff/BP_LevelInstance.PlayerChapsPos` _asbp_level_instance) _chapter))
      (`self.K2_SetActorLocation` _returnvalue _output false false)
      (`self.K2_SetActorRotation` (struct))
      (bind _returnvalue_2 (`GameplayStatics.GetActorOfClass` "/Game/Game/GameModesAndStuff/BP_DayManager.BP_DayManager_C"))
      (`/Game/Game/GameModesAndStuff/BP_DayManager.MakeDay` _returnvalue_2))
    (:`1`
      (`self.K2_SetActorLocation` _returnvalue _output false false)
      (bind _returnvalue_3 (`GameplayStatics.GetActorOfClass` "/Game/Game/GameModesAndStuff/BP_DayManager.BP_DayManager_C"))
      (`/Game/Game/GameModesAndStuff/BP_DayManager.MakeDawn` _returnvalue_3))
    (:`2`
      (`self.K2_SetActorLocation` _returnvalue _output false false)
      (bind _returnvalue_4 (`GameplayStatics.GetActorOfClass` "/Game/Game/GameModesAndStuff/BP_DayManager.BP_DayManager_C"))
      (`/Game/Game/GameModesAndStuff/BP_DayManager.MakeDawn` _returnvalue_4))))

(event `OpenCutscene1`
  (bind _asbp_level_instance (cast `/Game/Game/GameModesAndStuff/BP_LevelInstance` (`GameplayStatics.GetGameInstance`)))
  (set `/Game/Game/GameModesAndStuff/BP_LevelInstance.Chapter` 1 _asbp_level_instance)
  (set `/Game/Game/GameModesAndStuff/BP_LevelInstance.StartStory` true _asbp_level_instance)
  (`GameplayStatics.OpenLevel` "TVScene"))

(event `OpenCutscene2`
  (bind _asbp_level_instance (cast `/Game/Game/GameModesAndStuff/BP_LevelInstance` (`GameplayStatics.GetGameInstance`)))
  (set `/Game/Game/GameModesAndStuff/BP_LevelInstance.Chapter` 2 _asbp_level_instance)
  (set `/Game/Game/GameModesAndStuff/BP_LevelInstance.StartStory` true _asbp_level_instance)
  (`GameplayStatics.OpenLevel` "TVScene"))

(fn `UserConstructionScript`)