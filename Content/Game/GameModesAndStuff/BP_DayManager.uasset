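; BP_DayManager is an actor that sets the level's time-of-day lighting, switching it to night on BeginPlay.
; MakeNight rotates the Sun, dims and tints the Sun and Sky lights blue, and swaps the skybox material to a night instance.
; MakeDay, MakeDawn and MakeSunset only snap the Sun's rotation, and their calls in this graph are disconnected.
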(event `self.ReceiveBeginPlay`
  (`self.MakeNight`))

(event `MakeSunset`
  (`self.K2_SetActorRotation` (`self.Sun`) (struct :`Pitch` -175.0 :`Yaw` 30.0) false))

(event `MakeDay`
  (`self.K2_SetActorRotation` (`self.Sun`) (struct :`Pitch` -40.0 :`Yaw` 30.0) false))

(event `MakeDawn`
  (`self.K2_SetActorRotation` (`self.Sun`) (struct :`Pitch` -2.0 :`Yaw` 30.0) false))

(event `MakeNight`
  (bind _sun (`self.Sun`))
  (bind _sky (`self.Sky`))
  (`self.K2_SetActorRotation` _sun (struct :`Pitch` -40.0 :`Yaw` 30.0) false)
  (`LightComponent.SetIntensity` (`Light.LightComponent` _sun) 0.4)
  (`LightComponent.SetLightColor` (`Light.LightComponent` _sun) (struct :`G` 0.038774 :`B` 1.0 :`A` 1.0) true)
  (`SkyLightComponent.SetIntensity` (`SkyLight.LightComponent` _sky) 0.1)
  (`SkyLightComponent.SetLightColor` (`SkyLight.LightComponent` _sky) (struct :`R` 0.065357 :`B` 1.0 :`A` 1.0))
  (`PrimitiveComponent.SetMaterial` (`StaticMeshActor.StaticMeshComponent` (`self.Skybox`)) 0 "/Game/Fantastic_Village_Pack/materials/MI_skybox_night.MI_skybox_night"))

(fn `UserConstructionScript`)