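; Chapter 2 enemy NPC that talks to the player and starts an RPS minigame battle, destroying itself in other chapters.
; BeginPlay loads data-table dialogue, sphere overlap toggles a widget, and Tick bobs its shield on a sine wave.
; Finished dialogue saves temporary state and configures BP_RPSGameManager for combat.
; Win or loss swaps dialogue and restores state and control; winning also advances the shield-ball quest, while losing re-arms the battle.
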(event `ResetDialogues`
  (`KismetArrayLibrary.Array_Clear` (`self.DialoguesReady`))
  (bind _asbp_level_instance (cast `/Game/Game/GameModesAndStuff/BP_LevelInstance` (`GameplayStatics.GetGameInstance`) :!label _label))
  (if (== 2 (`/Game/Game/GameModesAndStuff/BP_LevelInstance.Chapter` _asbp_level_instance))
    (bind _outrownames (`DataTableFunctionLibrary.GetDataTableRowNames` (`|GetArrayItem` (`self.Dialogues`) (`self.DialogueIndex`))))
    (for _array_element _outrownames
      (bind _returnvalue (`|GetDataTableRow` (`|GetArrayItem` (`self.Dialogues`) (`self.DialogueIndex`)) _array_element)
        (:`then`
          (`KismetArrayLibrary.Array_Add` (`self.DialoguesReady`) _returnvalue))))
    (else
      (`self.K2_DestroyActor`))))

(event `self.ReceiveBeginPlay`
  (set `self.StartPosition` (`self.K2_GetActorLocation`))
  (`self.ToggleMarkerVisibility`)
  (goto _label))

(event `ToggleMarkerVisibility`
  (bind _marker (`self.MArker`))
  (if (`SceneComponent.IsVisible` _marker)
    (`SceneComponent.SetVisibility` _marker false false)
    (`ActorComponent.Deactivate` (`self.PS_QuadRibbon1`))
    (`ActorComponent.Deactivate` (`self.PS_QuadRibbon`))
    (else
      (`SceneComponent.SetVisibility` _marker true false)
      (`ActorComponent.Activate` (`self.PS_QuadRibbon1`) false)
      (`ActorComponent.Activate` (`self.PS_QuadRibbon`) false))))

(event `self.Sphere.OnComponentBeginOverlap`
  (params (OverlappedComponent :type "PrimitiveComponent Object Reference") (OtherActor :type "Actor Object Reference") (OtherComp :type "PrimitiveComponent Object Reference") (OtherBodyIndex :type Integer) (bFromSweep :type Boolean) (SweepResult :type "HitResult Structure (by ref)"))
  (cast `/Game/Game/Characters/BP_Boy` OtherActor)
  (`SceneComponent.SetVisibility` (`self.Widget`) true false))

(event `self.ReceiveTick`
  (params (DeltaSeconds :type "Float (single-precision)"))
  (`SceneComponent.K2_AddLocalOffset` (`self.shield3`) (`KismetMathLibrary.MakeVector` 0.0 0.0 (* (`KismetMathLibrary.Sin` (* (`GameplayStatics.GetRealTimeSeconds`) 10.0)) 0.5)) false false))

(event `self.Sphere.OnComponentEndOverlap`
  (params (OverlappedComponent :type "PrimitiveComponent Object Reference") (OtherActor :type "Actor Object Reference") (OtherComp :type "PrimitiveComponent Object Reference") (OtherBodyIndex :type Integer))
  (cast `/Game/Game/Characters/BP_Boy` OtherActor)
  (`SceneComponent.SetVisibility` (`self.Widget`) false false))

(event `self.DoSomethingOnFinish`
  (bind _asgm_basic_gameplay (cast `/Game/Game/GameModesAndStuff/GM_BasicGameplay` (`GameplayStatics.GetGameMode`)))
  (`/Game/Game/GameModesAndStuff/GM_BasicGameplay.SaveTemp` _asgm_basic_gameplay)
  (bind _returnvalue (`GameplayStatics.GetActorOfClass` "/Game/Game/RockPaperScissors/BP_RPSGameManager.BP_RPSGameManager_C"))
  (set `/Game/Game/RockPaperScissors/BP_RPSGameManager.RPSResults` "/Game/Game/RockPaperScissors/DT_RPSResults2.DT_RPSResults2" _returnvalue)
  (set `/Game/Game/RockPaperScissors/BP_RPSGameManager.MiniGameID` 2 _returnvalue)
  (set `/Game/Game/RockPaperScissors/BP_RPSGameManager.EnemyIconTexture` "/Game/Game/TV/Vigs/01.01" _returnvalue)
  (set `/Game/Game/RockPaperScissors/BP_RPSGameManager.Tutorial` false _returnvalue)
  (set `/Game/Game/RockPaperScissors/BP_RPSGameManager.WinningPoints` 8 _returnvalue)
  (`/Game/Game/RockPaperScissors/BP_RPSGameManager.StartCombat` _returnvalue self (`GameplayStatics.GetPlayerCharacter` 0))
  (`self.ToggleMarkerVisibility`)
  (bind _asgm_basic_gameplay_2 (cast `/Game/Game/GameModesAndStuff/GM_BasicGameplay` (`GameplayStatics.GetGameMode`)))
  (`/Game/Game/GameModesAndStuff/GM_BasicGameplay.SaveTemp` _asgm_basic_gameplay_2))

(event `self.Talk`
  (`self.StartDialogue`))

(event `StartDialogue`
  (bind _returnvalue (`GameplayStatics.GetPlayerController` 0))
  (bind _returnvalue_2 (`|CreateWidget` "/Game/Dialogue/WBP_DialogueBox.WBP_DialogueBox_C" (`GameplayStatics.GetPlayerController` 0) (`self.DialoguesReady`) (`self.StartBattle`) self))
  (bind _output_get (set `self.DialogueShown` _returnvalue_2))
  (`/Game/Dialogue/WBP_DialogueBox.UpdateDialogue` _output_get)
  (`UserWidget.AddToViewport` _output_get 0)
  (set `PlayerController.bShowMouseCursor` true _returnvalue)
  (`WidgetBlueprintLibrary.SetInputMode_UIOnlyEx` _returnvalue null "DoNotLock" true))

(event `self.WinEvent`
  (bind _returnvalue (`GameplayStatics.GetPlayerController` 0))
  (set `self.DialogueIndex` 3)
  (set `self.StartBattle` false)
  (`self.ResetDialogues`)
  (`self.StartDialogue`)
  (bind _asbp_level_instance (cast `/Game/Game/GameModesAndStuff/BP_LevelInstance` (`GameplayStatics.GetGameInstance`)))
  (`KismetArrayLibrary.Array_Set` (`/Game/Game/GameModesAndStuff/BP_LevelInstance.QuestTexts` _asbp_level_instance) (`/Game/Game/GameModesAndStuff/BP_LevelInstance.Chapter` _asbp_level_instance) "Get the shield ball back to Sergeant Wilson")
  (bind _returnvalue_2 (`GameplayStatics.GetActorOfClass` "/Game/Game/Characters/BP_Skelly.BP_Skelly_C"))
  (set `/Game/Game/Characters/BP_Skelly.QuestDone` true _returnvalue_2)
  (bind _asgm_basic_gameplay (cast `/Game/Game/GameModesAndStuff/GM_BasicGameplay` (`GameplayStatics.GetGameMode`)))
  (`/Game/Game/GameModesAndStuff/GM_BasicGameplay.ChangeQuestDeleg` _asgm_basic_gameplay)
  (bind _asgm_basic_gameplay_2 (cast `/Game/Game/GameModesAndStuff/GM_BasicGameplay` (`GameplayStatics.GetGameMode`) :!label _label_2))
  (`/Game/Game/GameModesAndStuff/GM_BasicGameplay.LoadTemp` _asgm_basic_gameplay_2)
  (`self.K2_SetActorLocation` (`self.StartPosition`))
  (`PlayerController.SetViewTargetWithBlend` _returnvalue (`GameplayStatics.GetPlayerCharacter` 0) 5.0 "VTBlend_Cubic" 0.0 false)
  (`WidgetBlueprintLibrary.SetInputMode_GameOnly` _returnvalue true)
  (`self.EnableInput` (`Controller.K2_GetPawn` _returnvalue) _returnvalue)
  (`SceneComponent.SetVisibility` (`self.shield3`) false false))

(event `self.LoseEvent`
  (set `self.DialogueIndex` 2)
  (set `self.StartBattle` false)
  (`self.ResetDialogues`)
  (`self.StartDialogue`)
  (`self.ToggleMarkerVisibility`)
  (set `self.StartBattle` true)
  (goto _label_2))

(fn `UserConstructionScript`)