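; BP_Skelly is a skeleton quest-giver NPC that shows a prompt widget near BP_Boy and destroys itself after chapter 2.
; It fills WBP_DialogueBox with DataTable rows picked by DialogueIndex.
; Talking at index 1 or higher arms BP_BigBad's battle and updates the lost-shield quest through the game instance and game mode.
; Once QuestDone, Talk reveals the shield and plays closing dialogue whose finish callback triggers the game mode's LastDialogue.
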(event `ResetDialogues`
  (`KismetArrayLibrary.Array_Clear` (`self.DialoguesReady`))
  (bind _asbp_level_instance (cast `/Game/Game/GameModesAndStuff/BP_LevelInstance` (`GameplayStatics.GetGameInstance`) :!label _label))
  (if (>= 2 (`/Game/Game/GameModesAndStuff/BP_LevelInstance.Chapter` _asbp_level_instance))
    (bind _outrownames (`DataTableFunctionLibrary.GetDataTableRowNames` (`|GetArrayItem` (`self.Dialogues`) (`self.DialogueIndex`))))
    (for _array_element _outrownames
      (bind _returnvalue (`|GetDataTableRow` (`|GetArrayItem` (`self.Dialogues`) (`self.DialogueIndex`)) _array_element)
        (:`then`
          (`KismetArrayLibrary.Array_Add` (`self.DialoguesReady`) _returnvalue))))
    (else
      (`self.K2_DestroyActor`))))

(event `self.ReceiveBeginPlay`
  (goto _label))

(event `self.Sphere.OnComponentBeginOverlap`
  (params (OverlappedComponent :type "PrimitiveComponent Object Reference") (OtherActor :type "Actor Object Reference") (OtherComp :type "PrimitiveComponent Object Reference") (OtherBodyIndex :type Integer) (bFromSweep :type Boolean) (SweepResult :type "HitResult Structure (by ref)"))
  (cast `/Game/Game/Characters/BP_Boy` OtherActor)
  (`SceneComponent.SetVisibility` (`self.Widget`) true false))

(event `self.Sphere.OnComponentEndOverlap`
  (params (OverlappedComponent :type "PrimitiveComponent Object Reference") (OtherActor :type "Actor Object Reference") (OtherComp :type "PrimitiveComponent Object Reference") (OtherBodyIndex :type Integer))
  (cast `/Game/Game/Characters/BP_Boy` OtherActor)
  (`SceneComponent.SetVisibility` (`self.Widget`) false false))

(event `self.Talk`
  (if (`self.QuestDone`)
    (`SceneComponent.SetVisibility` (`self.shield3`) true false)
    (`self.CloseGame`)
    (else
      (`self.StartDialogue`)
      (if (>= (`self.DialogueIndex`) 1)
        (if (not (`self.QuestDone`))
          (bind _returnvalue (`GameplayStatics.GetActorOfClass` "/Game/Game/Enemies/BP_BigBad.BP_BigBad_C"))
          (set `/Game/Game/Enemies/BP_BigBad.DialogueIndex` 1 _returnvalue)
          (`/Game/Game/Enemies/BP_BigBad.ToggleMarkerVisibility` _returnvalue)
          (`/Game/Game/Enemies/BP_BigBad.ResetDialogues` _returnvalue)
          (set `/Game/Game/Enemies/BP_BigBad.StartBattle` true _returnvalue)
          (bind _asbp_level_instance (cast `/Game/Game/GameModesAndStuff/BP_LevelInstance` (`GameplayStatics.GetGameInstance`)))
          (`KismetArrayLibrary.Array_Set` (`/Game/Game/GameModesAndStuff/BP_LevelInstance.QuestTexts` _asbp_level_instance) (`/Game/Game/GameModesAndStuff/BP_LevelInstance.Chapter` _asbp_level_instance) "Recover Seargent Wilson's lost shield! He usually likes to roam around warm places in town")
          (bind _asgm_basic_gameplay (cast `/Game/Game/GameModesAndStuff/GM_BasicGameplay` (`GameplayStatics.GetGameMode`)))
          (`/Game/Game/GameModesAndStuff/GM_BasicGameplay.ChangeQuestDeleg` _asgm_basic_gameplay))))))

(event `StartDialogue`
  (bind _returnvalue (`GameplayStatics.GetPlayerController` 0))
  (bind _returnvalue_2 (`|CreateWidget` "/Game/Dialogue/WBP_DialogueBox.WBP_DialogueBox_C" (`GameplayStatics.GetPlayerController` 0) (`self.DialoguesReady`) false null "/Game/Game/Audio/Sources/ghostvoice.ghostvoice"))
  (bind _output_get (set `self.DialogueShown` _returnvalue_2))
  (`/Game/Dialogue/WBP_DialogueBox.UpdateDialogue` _output_get)
  (`UserWidget.AddToViewport` _output_get 0)
  (set `PlayerController.bShowMouseCursor` true _returnvalue)
  (`WidgetBlueprintLibrary.SetInputMode_UIOnlyEx` _returnvalue null "DoNotLock" true))

(event `/Game/Dialogue/BI_DialogueInterface.DoSomethingOnFinish`
  (bind _asgm_basic_gameplay (cast `/Game/Game/GameModesAndStuff/GM_BasicGameplay` (`GameplayStatics.GetGameMode`)))
  (`/Game/Game/GameModesAndStuff/GM_BasicGameplay.LastDialogue` _asgm_basic_gameplay))

(event `CloseGame`
  (bind _returnvalue (`GameplayStatics.GetPlayerController` 0))
  (`KismetArrayLibrary.Array_Clear` (`self.DialoguesReady`))
  (bind _outrownames (`DataTableFunctionLibrary.GetDataTableRowNames` (`|GetArrayItem` (`self.Dialogues`) 2)))
  (for _array_element _outrownames
    (bind _returnvalue_2 (`|GetDataTableRow` (`|GetArrayItem` (`self.Dialogues`) 2) _array_element)
      (:`then`
        (`KismetArrayLibrary.Array_Add` (`self.DialoguesReady`) _returnvalue_2)
        (bind _returnvalue_3 (`|CreateWidget` "/Game/Dialogue/WBP_DialogueBox.WBP_DialogueBox_C" (`GameplayStatics.GetPlayerController` 0) (`self.DialoguesReady`) true self "/Game/Game/Audio/Sources/ghostvoice.ghostvoice"))
        (bind _output_get (set `self.DialogueShown` _returnvalue_3))
        (`/Game/Dialogue/WBP_DialogueBox.UpdateDialogue` _output_get)
        (`UserWidget.AddToViewport` _output_get 0)
        (set `PlayerController.bShowMouseCursor` true _returnvalue)
        (`WidgetBlueprintLibrary.SetInputMode_UIOnlyEx` _returnvalue null "DoNotLock" true)))))

(fn `UserConstructionScript`)