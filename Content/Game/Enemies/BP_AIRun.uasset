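; AI controller Blueprint that keeps its enemy pawn wandering to random reachable points within a large radius of its current position.
; BeginPlay starts NewPath, which calls AIMoveTo and repeats itself on success, with no retry if the point search or move fails.
; The random-point query is re-evaluated at each use, so the debug sphere it draws may not mark the actual destination.
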(event `self.ReceiveBeginPlay`
  (`self.NewPath`))

(event `NewPath`
  (bind (_randomlocation _returnvalue) (`NavigationSystemV1.K2_GetRandomReachablePointInRadius` (`self.K2_GetActorLocation` (`self.K2_GetPawn`)) 10000.0 null null))
  (`KismetSystemLibrary.DrawDebugSphere` _randomlocation 100.0 12 (struct :`R` 1.0 :`G` 1.0 :`B` 1.0 :`A` 1.0) 10.0)
  (if _returnvalue
    (`|AIMoveTo` (`self.K2_GetPawn`) _randomlocation null 100.0
      (:`OnSuccess`
        (`self.NewPath`)))))

(fn `UserConstructionScript`)