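; BP_Biblioteca is a trigger actor that starts the first cutscene during chapter 0.
; On BeginPlay it reads Chapter from the BP_LevelInstance game instance and destroys itself if the chapter is not 0.
; When BP_Boy overlaps its Sphere, it calls OpenCutscene1 on the GM_BasicGameplay game mode, with no guard against repeat triggering.
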(event `self.ReceiveBeginPlay`
  (bind _asbp_level_instance (cast `/Game/Game/GameModesAndStuff/BP_LevelInstance` (`GameplayStatics.GetGameInstance`)))
  (if (not (== (`/Game/Game/GameModesAndStuff/BP_LevelInstance.Chapter` _asbp_level_instance) 0))
    (`self.K2_DestroyActor`)))

(event `self.Sphere.OnComponentBeginOverlap`
  (params (OverlappedComponent :type "PrimitiveComponent Object Reference") (OtherActor :type "Actor Object Reference") (OtherComp :type "PrimitiveComponent Object Reference") (OtherBodyIndex :type Integer) (bFromSweep :type Boolean) (SweepResult :type "HitResult Structure (by ref)"))
  (cast `/Game/Game/Characters/BP_Boy` OtherActor)
  (bind _asgm_basic_gameplay (cast `/Game/Game/GameModesAndStuff/GM_BasicGameplay` (`GameplayStatics.GetGameMode`)))
  (`/Game/Game/GameModesAndStuff/GM_BasicGameplay.OpenCutscene1` _asgm_basic_gameplay))

(fn `UserConstructionScript`)