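; Rock-paper-scissors minigame enemy that starts combat when BP_Boy overlaps its box, initializing BP_BattleManager and opening WBP_RPS_UI.
; SetChoices pairs the player's pick with a random enemy pick, then TurnPlaying spawns pumpkin, candy or scissor items and explodes the loser's.
; CheckTurnWinner scores the turn from the RPSResults data table, adding streak-based bonuses or penalties per MiniGameID.
; CheckGameWinner compares points to WinningPoints and notifies the enemy of the result.
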(event `StartCombat`
  (params (Enemy :type "Actor Object Reference") (Player :type "Actor Object Reference"))
  (bind _returnvalue (`GameplayStatics.GetPlayerController` 0))
  (bind _returnvalue_2 (`GameplayStatics.GetActorOfClass` "/Game/Game/Combat/BP_BattleManager.BP_BattleManager_C"))
  (set `self.Enemy` Enemy)
  (`/Game/Game/Combat/BP_BattleManager.InitializeCombat` _returnvalue_2 Enemy Player)
  (bind _returnvalue_3 (`|CreateWidget` "/Game/Game/UI/WBP_RPS_UI.WBP_RPS_UI_C" null self null))
  (set `/Game/Game/UI/WBP_RPS_UI.EnemyIconTexture` (`self.EnemyIconTexture`) _returnvalue_3)
  (set `/Game/Game/UI/WBP_RPS_UI.Tutorial` (`self.Tutorial`) _returnvalue_3)
  (`UserWidget.AddToViewport` _returnvalue_3 0)
  (set `/Game/Game/UI/WBP_RPS_UI.WinningPoints` (`self.WinningPoints`) _returnvalue_3)
  (set `self.PlayerPoints` 0)
  (set `self.EnemyPoints` 0)
  (set `PlayerController.bShowMouseCursor` true _returnvalue)
  (`WidgetBlueprintLibrary.SetInputMode_UIOnlyEx` _returnvalue null "DoNotLock" true))

(event `self.Box.OnComponentBeginOverlap`
  (params (OverlappedComponent :type "PrimitiveComponent Object Reference") (OtherActor :type "Actor Object Reference") (OtherComp :type "PrimitiveComponent Object Reference") (OtherBodyIndex :type Integer) (bFromSweep :type Boolean) (SweepResult :type "HitResult Structure (by ref)"))
  (bind _asbp_boy (cast `/Game/Game/Characters/BP_Boy` OtherActor))
  (`self.StartCombat` self _asbp_boy))

(event `self.ReceiveActorBeginOverlap`
  (params (OtherActor :type "Actor Object Reference")))

(event `self.ReceiveTick`
  (params (DeltaSeconds :type "Float (single-precision)")))

(event `self.ReceiveBeginPlay`)

(event `TurnPlaying`
  (bind _returnvalue (`GameplayStatics.GetPlayerCharacter` 0))
  (bind _enemy (`self.Enemy`))
  (bind _enemyspawn (`self.EnemySpawn`))
  (bind _playerspawn (`self.PlayerSpawn`))
  (bind _returnvalue_2 (`KismetMathLibrary.MakeTransform` (+ (`self.K2_GetActorLocation` _enemy) (* (`self.GetActorForwardVector` _enemy) 200))))
  (bind _returnvalue_3 (`KismetMathLibrary.MakeTransform` (+ (`self.K2_GetActorLocation` _returnvalue) (* (`self.GetActorForwardVector` _returnvalue) 200))))
  (`self.DisableInput` (`GameplayStatics.GetPlayerCharacter` 0) (`GameplayStatics.GetPlayerController` 0))
  (switch `/Game/Game/RockPaperScissors/E_RPSChoices` (`self.PlayerChoice`)
    (:`NewEnumerator0`
      (bind _returnvalue_4 (`|SpawnActorFromClass` "/Game/Game/OtherBPs/BP_PumpkinItem.BP_PumpkinItem_C" _returnvalue_3 "Undefined" "MultiplyWithRoot" null null))
      (set `self.PlayerSpawn` _returnvalue_4))
    (:`NewEnumerator1`
      (bind _returnvalue_5 (`|SpawnActorFromClass` "/Game/Game/OtherBPs/BP_CandyItem.BP_CandyItem_C" _returnvalue_3 "Undefined" "MultiplyWithRoot" null null))
      (set `self.PlayerSpawn` _returnvalue_5))
    (:`NewEnumerator2`
      (bind _returnvalue_6 (`|SpawnActorFromClass` "/Game/Game/OtherBPs/BP_ScissorItem1.BP_ScissorItem1_C" _returnvalue_3 "Undefined" "MultiplyWithRoot" null null))
      (set `self.PlayerSpawn` _returnvalue_6)))
  (switch `/Game/Game/RockPaperScissors/E_RPSChoices` (`self.EnemyChoice`)
    (:`NewEnumerator0`
      (bind _returnvalue_7 (`|SpawnActorFromClass` "/Game/Game/OtherBPs/BP_PumpkinItem.BP_PumpkinItem_C" _returnvalue_2 "Undefined" "MultiplyWithRoot" null null))
      (set `self.EnemySpawn` _returnvalue_7))
    (:`NewEnumerator1`
      (bind _returnvalue_8 (`|SpawnActorFromClass` "/Game/Game/OtherBPs/BP_CandyItem.BP_CandyItem_C" _returnvalue_2 "Undefined" "MultiplyWithRoot" null null))
      (set `self.EnemySpawn` _returnvalue_8))
    (:`NewEnumerator2`
      (bind _returnvalue_9 (`|SpawnActorFromClass` "/Game/Game/OtherBPs/BP_ScissorItem1.BP_ScissorItem1_C" _returnvalue_2 "Undefined" "MultiplyWithRoot" null null))
      (set `self.EnemySpawn` _returnvalue_9)))
  (`KismetSystemLibrary.Delay` 1.0)
  (switch `/Game/Game/RockPaperScissors/E_RPSOutcomes` (`self.Outcome`)
    (:`NewEnumerator0`
      (`GameplayStatics.SpawnEmitterAtLocation` "/Game/Realistic_Starter_VFX_Pack_Vol2/Particles/Explosion/P_Explosion_Big_A.P_Explosion_Big_A" (`self.K2_GetActorLocation` _enemyspawn))
      (`self.K2_DestroyActor` _enemyspawn)
      (`KismetSystemLibrary.Delay` 1.0)
      (`self.K2_DestroyActor` (`self.PlayerSpawn`))
      (`self.EnableInput` (`GameplayStatics.GetPlayerCharacter` 0) (`GameplayStatics.GetPlayerController` 0) :!label _label))
    (:`NewEnumerator1`
      (`GameplayStatics.SpawnEmitterAtLocation` "/Game/Realistic_Starter_VFX_Pack_Vol2/Particles/Explosion/P_Explosion_Big_A.P_Explosion_Big_A" (`self.K2_GetActorLocation` _playerspawn) (struct) (1.0 10.0 1.0))
      (`self.K2_DestroyActor` _playerspawn)
      (`KismetSystemLibrary.Delay` 1.0)
      (`self.K2_DestroyActor` (`self.EnemySpawn`))
      (goto _label))
    (:`NewEnumerator2`
      (`KismetSystemLibrary.Delay` 1.0)
      (`self.K2_DestroyActor` (`self.PlayerSpawn`))
      (`KismetSystemLibrary.Delay` 1.0)
      (`self.K2_DestroyActor` (`self.EnemySpawn`)))))

(fn `CheckGameWinner`
  (returns (Winner :type "/Game/Game/RockPaperScissors/E_RPSWinner Enum"))
  (bind _playerpoints (`self.PlayerPoints`))
  (bind _enemypoints (`self.EnemyPoints`))
  (bind _winningpoints (`self.WinningPoints`))
  (bind _enemy (`self.Enemy`))
  (bind _returnvalue (>= _enemypoints _winningpoints))
  (if (>= _playerpoints _winningpoints)
    (if _returnvalue
      (if (>= _playerpoints _enemypoints)
        (`KismetSystemLibrary.PrintText` "Player wins!" :!label _label)
        (message `/Game/Game/RockPaperScissors/BP_Combat.WinEvent` _enemy)
        (return "NewEnumerator0")
        (else
          _))
      (else
        (goto _label)))
    (elif _returnvalue
      _
      (else
        (return "NewEnumerator2"))))
  (`KismetSystemLibrary.PrintText` "Enemy wins :(")
  (message `/Game/Game/RockPaperScissors/BP_Combat.LoseEvent` _enemy)
  (return "NewEnumerator1"))

(fn `CheckTurnWinner`
  (returns (Outcome :type "/Game/Game/RockPaperScissors/E_RPSOutcomes Enum") (PlayerPoints :type Integer) (EnemyPoints :type Integer))
  (bind _returnvalue (`self.ChoicesToRow` (`self.PlayerChoice`) (`self.EnemyChoice`)))
  (bind _returnvalue_2 (`|GetDataTableRow` (`self.RPSResults`) _returnvalue)
    (:`then`
      (bind (_outcome _playerpoints _enemypoints) (`self.UpdatePoints` _returnvalue_2))
      (set `self.PrevOutcome` (`self.Outcome`))
      (bind _output_get (set `self.Outcome` _outcome))
      (`self.PrintPoints` _playerpoints _enemypoints)
      (return _output_get _playerpoints _enemypoints))))

(fn `ChoicesToRow`
  (params (PlayerChoice :type "/Game/Game/RockPaperScissors/E_RPSChoices Enum" :default "NewEnumerator0") (EnemyChoice :type "/Game/Game/RockPaperScissors/E_RPSChoices Enum" :default "NewEnumerator0"))
  (returns (ReturnValue :type Name))
  (return (`KismetStringLibrary.Conv_StringToName` (`KismetStringLibrary.Concat_StrStr` (`|GetEnumeratorNameAsString` PlayerChoice) (`|GetEnumeratorNameAsString` EnemyChoice)))))

(fn `PrintPoints`
  (params (Value :type Integer) (Value2 :type Integer))
  (`KismetSystemLibrary.PrintText` (`KismetTextLibrary.Conv_StringToText` (`KismetStringLibrary.Concat_StrStr` "Player points: " (`KismetTextLibrary.Conv_TextToString` (`KismetTextLibrary.Conv_IntToText` Value)))))
  (`KismetSystemLibrary.PrintText` (`KismetTextLibrary.Conv_StringToText` (`KismetStringLibrary.Concat_StrStr` "Enemy points: " (`KismetTextLibrary.Conv_TextToString` (`KismetTextLibrary.Conv_IntToText` Value2))))))

(fn `RunExtraRules`
  (returns (PlayerPointsModifier :type Integer))
  (bind _minigameid (`self.MiniGameID`))
  (if (`self.IsValid`)
    (if (== _minigameid 2)
      (switch `/Game/Game/RockPaperScissors/E_RPSOutcomes` (`self.Outcome`)
        (:`NewEnumerator0`
          (if (and (`|EnumEquality` (`self.PrevOutcome`) "NewEnumerator0") (`|EnumEquality` (`self.PlayerChoice`) "NewEnumerator2") (`|EnumEquality` (`self.PrevPlayerChoice`) "NewEnumerator2"))
            (return 1)
            (else
              _)))
        (:`NewEnumerator1`
          (if (`|EnumEquality` (`self.PrevOutcome`) "NewEnumerator1")
            (return -1)
            (else
              _)))
        (:`NewEnumerator2`
          _))
      (return 0)
      (else
        (if (== _minigameid 3)
          (if (and (`|EnumEquality` (`self.PrevOutcome`) "NewEnumerator0") (`|EnumEquality` (`self.Outcome`) "NewEnumerator0") (`|EnumEquality` (`self.PlayerChoice`) (`self.PrevPlayerChoice`)))
            (return -1)
            (else
              _))
          (elif (== _minigameid 4)
            (if (and (`|EnumEquality` (`self.PrevOutcome`) "NewEnumerator1") (`|EnumEquality` (`self.Outcome`) "NewEnumerator0") (`|EnumEquality` (`self.PlayerChoice`) (`self.PrevPlayerChoice`)))
              (return 2)
              (else
                (return 0)))
            (else
              _)))
        (return 0)))
    (else
      (set `self.IsValid` true)
      (return 0))))

(fn `SetChoices`
  (params (PlayerChoice :type "/Game/Game/RockPaperScissors/E_RPSChoices Enum" :default "NewEnumerator0"))
  (set `self.PrevPlayerChoice` (`self.PlayerChoice`))
  (bind _output_get (set `self.PlayerChoice` PlayerChoice))
  (bind _output_get_2 (set `self.EnemyChoice` (`KismetArrayLibrary.Array_Random` (`self.RPSChoices`))))
  (`KismetSystemLibrary.PrintString` (`KismetStringLibrary.Concat_StrStr` "Player: " (`|GetEnumeratorNameAsString` _output_get)))
  (`KismetSystemLibrary.PrintString` (`KismetStringLibrary.Concat_StrStr` "Enemy: " (`|GetEnumeratorNameAsString` _output_get_2)))
  (`self.TurnPlaying`)
  (return))

(fn `UpdatePoints`
  (params (ST_RPSResults :type "/Game/Game/RockPaperScissors/ST_RPSResults Structure (by ref)"))
  (returns (Outcome :type "/Game/Game/RockPaperScissors/E_RPSOutcomes Enum") (PlayerPoints :type Integer) (EnemyPoints :type Integer))
  (bind (_playerchoice _enemychoice _playerpoints _enemypoints _outcome) (break `/Game/Game/RockPaperScissors/ST_RPSResults` ST_RPSResults))
  (bind _playerpointsmodifier (`self.RunExtraRules`))
  (if (!= _playerpointsmodifier 0)
    (set `self.IsValid` false))
  (bind _output_get (set `self.PlayerPoints` (+ _playerpointsmodifier (`KismetMathLibrary.Max` (+ (`self.PlayerPoints`) _playerpoints)))))
  (bind _output_get_2 (set `self.EnemyPoints` (`KismetMathLibrary.Max` (+ _enemypoints (`self.EnemyPoints`)))))
  (return _outcome _output_get _output_get_2))

(fn `UserConstructionScript`)