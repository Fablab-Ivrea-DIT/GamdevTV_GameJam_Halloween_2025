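; Kitty NPC that shows a prompt widget while BP_Boy is in range and opens dialogue when talked to.
; BeginPlay caches the current chapter's DataTable rows, which Talk feeds into WBP_DialogueBox with UI-only input.
; In chapter 1, once Bullo, Frog and Brush flags are all false, Talk instead loads DialoguesExtra by Dialogues[0] row names, creating a box per found row.
; That dialogue's finish hook opens Cutscene 2 through the game mode.
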(event `self.ReceiveBeginPlay`
  (bind _asbp_level_instance (cast `/Game/Game/GameModesAndStuff/BP_LevelInstance` (`GameplayStatics.GetGameInstance`)))
  (bind _chapter (`/Game/Game/GameModesAndStuff/BP_LevelInstance.Chapter` _asbp_level_instance))
  (bind _outrownames (`DataTableFunctionLibrary.GetDataTableRowNames` (`|GetArrayItem` (`self.Dialogues`) _chapter)))
  (for _array_element _outrownames
    (bind _returnvalue (`|GetDataTableRow` (`|GetArrayItem` (`self.Dialogues`) _chapter) _array_element)
      (:`then`
        (`KismetArrayLibrary.Array_Add` (`self.DialoguesReady`) _returnvalue)))))

(event `self.Sphere.OnComponentBeginOverlap`
  (params (OverlappedComponent :type "PrimitiveComponent Object Reference") (OtherActor :type "Actor Object Reference") (OtherComp :type "PrimitiveComponent Object Reference") (OtherBodyIndex :type Integer) (bFromSweep :type Boolean) (SweepResult :type "HitResult Structure (by ref)"))
  (cast `/Game/Game/Characters/BP_Boy` OtherActor)
  (`SceneComponent.SetVisibility` (`self.Widget`) true false))

(event `self.Sphere.OnComponentEndOverlap`
  (params (OverlappedComponent :type "PrimitiveComponent Object Reference") (OtherActor :type "Actor Object Reference") (OtherComp :type "PrimitiveComponent Object Reference") (OtherBodyIndex :type Integer))
  (cast `/Game/Game/Characters/BP_Boy` OtherActor)
  (`SceneComponent.SetVisibility` (`self.Widget`) false false))

(event `self.Talk`
  (bind _asbp_level_instance (cast `/Game/Game/GameModesAndStuff/BP_LevelInstance` (`GameplayStatics.GetGameInstance`)))
  (bind _returnvalue (== (`/Game/Game/GameModesAndStuff/BP_LevelInstance.Chapter` _asbp_level_instance) 1))
  (if _returnvalue
    (bind _returnvalue_2 (`GameplayStatics.GetActorOfClass` "/Game/Game/Enemies/BP_Bullo.BP_Bullo_C"))
    (bind _returnvalue_3 (`GameplayStatics.GetActorOfClass` "/Game/Game/OtherBPs/BP_Frog.BP_Frog_C"))
    (bind _returnvalue_4 (`GameplayStatics.GetActorOfClass` "/Game/Game/OtherBPs/BP_Brush.BP_Brush_C"))
    (if (and _returnvalue (not (or (`/Game/Game/Enemies/BP_Bullo.StartBattle` _returnvalue_2) (`/Game/Game/OtherBPs/BP_Frog.ShouldPick` _returnvalue_3) (`/Game/Game/OtherBPs/BP_Brush.ShouldPick` _returnvalue_4))))
      (`self.StartConclusiveDialogueChap1`)
      (else
        (`self.StartDialogue` :!label _label)))
    (else
      (goto _label))))

(event `StartDialogue`
  (bind _returnvalue (`GameplayStatics.GetPlayerController` 0))
  (bind _returnvalue_2 (`|CreateWidget` "/Game/Dialogue/WBP_DialogueBox.WBP_DialogueBox_C" (`GameplayStatics.GetPlayerController` 0) (`self.DialoguesReady`) false null))
  (bind _output_get (set `self.DialogueShown` _returnvalue_2))
  (`/Game/Dialogue/WBP_DialogueBox.UpdateDialogue` _output_get)
  (`UserWidget.AddToViewport` _output_get 0)
  (set `PlayerController.bShowMouseCursor` true _returnvalue)
  (`WidgetBlueprintLibrary.SetInputMode_UIOnlyEx` _returnvalue null "DoNotLock" true))

(event `self.DoSomethingOnFinish`
  (bind _asgm_basic_gameplay (cast `/Game/Game/GameModesAndStuff/GM_BasicGameplay` (`GameplayStatics.GetGameMode`)))
  (`/Game/Game/GameModesAndStuff/GM_BasicGameplay.OpenCutscene2` _asgm_basic_gameplay))

(event `StartConclusiveDialogueChap1`
  (bind _returnvalue (`GameplayStatics.GetPlayerController` 0))
  (`KismetArrayLibrary.Array_Clear` (`self.DialoguesReady`))
  (bind _outrownames (`DataTableFunctionLibrary.GetDataTableRowNames` (`|GetArrayItem` (`self.Dialogues`))))
  (for _array_element _outrownames
    (bind _returnvalue_2 (`|GetDataTableRow` (`|GetArrayItem` (`self.DialoguesExtra`)) _array_element)
      (:`then`
        (`KismetArrayLibrary.Array_Add` (`self.DialoguesReady`) _returnvalue_2)
        (bind _returnvalue_3 (`|CreateWidget` "/Game/Dialogue/WBP_DialogueBox.WBP_DialogueBox_C" (`GameplayStatics.GetPlayerController` 0) (`self.DialoguesReady`) true self))
        (bind _output_get (set `self.DialogueShown` _returnvalue_3))
        (`/Game/Dialogue/WBP_DialogueBox.UpdateDialogue` _output_get)
        (`UserWidget.AddToViewport` _output_get 0)
        (set `PlayerController.bShowMouseCursor` true _returnvalue)
        (`WidgetBlueprintLibrary.SetInputMode_UIOnlyEx` _returnvalue null "DoNotLock" true)))))

(fn `UserConstructionScript`)